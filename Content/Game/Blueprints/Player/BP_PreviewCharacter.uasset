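; BP_PreviewCharacter is a preview character with a camera on a spring arm that can be rotated and zoomed.
; RotateCamPreview yaws the spring arm by the input value.
; ZoomCamPreview clamps a target zoom, interpolates the arm length toward it, and lowers the socket offset as the arm extends.
; Interpolation only steps when the zoom event is called, as Tick is empty.
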(event `Rotate Cam Preview`
  (params (Value :type "Float (double-precision)"))
  (`SceneComponent.K2_AddLocalRotation` (`self.SpringArm`) (`KismetMathLibrary.MakeRotator` 0.0 0.0 Value) false false))

(event `Zoom Cam Preview`
  (params (Value :type "Float (double-precision)"))
  (set `self.Target Zoom` (`KismetMathLibrary.FClamp` (+ (* (* Value -1.0) (`self.ZoomSpeed`)) (`self.Target Zoom`)) (`self.MinZoom`) (`self.MaxZoom`)))
  (bind _output_get (set `self.Current Zoom` (`KismetMathLibrary.FInterpTo` (`self.Current Zoom`) (`self.Target Zoom`) (`GameplayStatics.GetWorldDeltaSeconds`) 15.0)))
  (set `SpringArmComponent.TargetArmLength` _output_get (`self.SpringArm`))
  (set `SpringArmComponent.SocketOffset` (`KismetMathLibrary.MakeVector` 0.0 0.0 (`KismetMathLibrary.Lerp` 0.0 -60.0 (/ (- (`self.Current Zoom`) (`self.MinZoom`)) (- (`self.MaxZoom`) (`self.MinZoom`))))) (`self.SpringArm`)))

(event `self.ReceiveTick`
  (params (DeltaSeconds :type "Float (single-precision)")))

(fn `UserConstructionScript`)